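; BP_MonsterTest is a test monster character that reacts visually to taking damage.
; AnyDamage briefly swaps both mesh materials to a hit flash, then after a short delay restores them, stops the attack montage, plays the damage montage and prints a debug message.
; Tick rotates the HP bar component to face the player camera.
; GetHit is an empty event, and a leftover attacker-direction calculation is unconnected.
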(event `GetHit`
  (params (Attacker :type "Actor Object Reference")))

(event `self.ReceiveAnyDamage`
  (params (Damage :type "Float (single-precision)") (DamageType :type "DamageType Object Reference") (InstigatedBy :type "Controller Object Reference") (DamageCauser :type "Actor Object Reference"))
  (`PrimitiveComponent.SetMaterial` (`self.Mesh`) 0 "/Game/test/Damage/M_HitFlash.M_HitFlash")
  (`PrimitiveComponent.SetMaterial` (`self.Mesh`) 1 "/Game/test/Damage/M_HitFlash.M_HitFlash")
  (`KismetSystemLibrary.Delay` 0.2)
  (`PrimitiveComponent.SetMaterial` (`self.Mesh`) 0 "/Game/test/mob/mob_rigged_2_Material__37_BaseColor_Mat.mob_rigged_2_Material__37_BaseColor_Mat")
  (`PrimitiveComponent.SetMaterial` (`self.Mesh`) 1 "/Game/test/mob/mob_rigged_2_Material__25_BaseColor_Mat.mob_rigged_2_Material__25_BaseColor_Mat")
  (`self.StopAnimMontage` "/Game/animation/mob/Mob_Attack_New_Montage.Mob_Attack_New_Montage")
  (`self.PlayAnimMontage` "/Game/animation/mob/Mob_Damage_Montage.Mob_Damage_Montage")
  (`KismetSystemLibrary.PrintString` "get damaged" true true (struct :`R` 1.0 :`G` 0.998857 :`A` 1.0) 5.0))

(event `self.ReceiveTick`
  (params (DeltaSeconds :type "Float (single-precision)"))
  (bind _hpbarcomponent (`self.HPBarComponent`))
  (`SceneComponent.K2_SetWorldRotation` _hpbarcomponent (`KismetMathLibrary.FindLookAtRotation` (`SceneComponent.K2_GetComponentLocation` _hpbarcomponent) (`PlayerCameraManager.GetCameraLocation` (`GameplayStatics.GetPlayerCameraManager` 0))) false false))

(fn `UserConstructionScript`)