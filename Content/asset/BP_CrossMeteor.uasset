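; BP_CrossMeteor is a falling skill projectile, a cross meteor that impacts, lingers, then clears itself away.
; On Hit it stops its ProjectileMovement and spawns Niagara sparks at the impact point.
; After a short delay it disables the mesh's collision and sinks it with MoveComponentTo, using the actor's world transform, offset downward, as the relative target.
; The actor is destroyed when the move finishes, followed by a debug print.
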(event `self.ReceiveHit`
  (params (MyComp :type "PrimitiveComponent Object Reference") (Other :type "Actor Object Reference") (OtherComp :type "PrimitiveComponent Object Reference") (bSelfMoved :type Boolean) (HitLocation :type "Vector Structure") (HitNormal :type "Vector Structure") (NormalImpulse :type "Vector Structure") (Hit :type "HitResult Structure (by ref)"))
  (bind _crossmeteor (`self.CrossMeteor`))
  ; 에셋 떨구는 스킬 노드ㅜ
  (`MovementComponent.StopMovementImmediately` (`self.ProjectileMovement`))
  (`NiagaraFunctionLibrary.SpawnSystemAtLocation` "/Game/Effect/NS_Sparks.NS_Sparks" HitLocation)
  (`KismetSystemLibrary.Delay` 3.0)
  (`PrimitiveComponent.SetCollisionEnabled` _crossmeteor "NoCollision")
  (`KismetSystemLibrary.MoveComponentTo` _crossmeteor (- (`self.K2_GetActorLocation`) (0.0 0.0 500.0)) (`self.K2_GetActorRotation`) false false 3.0)
  (`self.K2_DestroyActor`)
  (`KismetSystemLibrary.PrintString` "cross work"))

(fn `UserConstructionScript`)